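; BP_Animal is an AI-driven animal character that passes its own behavior settings to its Blackboard.
; On BeginPlay it writes its sociality, alpha status and a wait time, randomly scaled around the base value so individuals vary.
; A SwitchSpeed function toggles the movement component's max walk speed between walking and running speeds.
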(event EventBeginPlay
  (bind _returnvalue (AI|GetBlackboard 0))
  (AI|Components|Blackboard|SetValueasEnum _returnvalue (Utilities|Name|MakeLiteralName "SocialityKey") (Variables|Default|GetSociality))
  (AI|Components|Blackboard|SetValueasBool _returnvalue (Utilities|Name|MakeLiteralName "ifAlphaKey") (Variables|Default|GetifAlpha))
  (AI|Components|Blackboard|SetValueasFloat _returnvalue (Utilities|Name|MakeLiteralName "WaitTimeKey") (* (Math|Random|RandomFloatinRange 0.8 1.25) (Variables|Default|GetWaitTime))))

(fn ConstructionScript)

(fn SwitchSpeed
  (bind _charactermovement (Variables|Character|GetCharacterMovement))
  (if (== (Variables|/Script/Engine.CharacterMovementComponent|GetMaxWalkSpeed (Variables|Character|GetCharacterMovement)) (Variables|Default|GetWalkSpeed))
    (Variables|/Script/Engine.CharacterMovementComponent|SetMaxWalkSpeed _charactermovement (Variables|Default|GetRunSpeed))
    (else
      (Variables|/Script/Engine.CharacterMovementComponent|SetMaxWalkSpeed _charactermovement (Variables|Default|GetWalkSpeed)))))