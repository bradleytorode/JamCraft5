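; BP_AnimalManager is a manager Blueprint that tracks animals in the level, currently only pigs.
; On BeginPlay, OrganiseAnimals gathers every BP_Pig actor into a Pigs array without duplicates.
; FindAlpha takes an animal class and, for pigs, returns the first one in that array flagged as alpha.
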(event EventBeginPlay
  (CallFunction|OrganiseAnimals))

(fn ConstructionScript)

(fn OrganiseAnimals
  ;[1 1 1] Pigs
  (bind _outactors (Actor|GetAllActorsOfClass "/Game/AI/Animals/Instances/BP_Pig.BP_Pig_C"))
  (for _array_element _outactors
    (Utilities|Array|AddUnique (Variables|Default|GetPigs) _array_element)))

(fn FindAlpha
  (params (AnimalClass :type BP%20Animal%20Class%20Reference))
  (if (== AnimalClass "/Game/AI/Animals/Instances/BP_Pig.BP_Pig_C")
    (bind _array_element (Utilities|Array|ForEachLoopwithBreak (Variables|Default|GetPigs))
      (:LoopBody
        (if (Variables|/Game/AI/Animals/BP_Animal.BP_Animal_C|GetifAlpha _array_element)
          (return _array_element))))))